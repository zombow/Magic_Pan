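; BP_Enemy is an enemy with a simple Idle, Move and Attack state machine evaluated on Tick.
; A Sphere overlap with an actor whose display name is "MYHarry" switches it to Move.
; Move calls AI MoveTo toward the overlapped actor each tick, switching to Attack on success or failure.
; Attack is a placeholder debug print and jump, returning to Move when the target is far enough away.
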(event `self.ReceiveTick`
  (params (DeltaSeconds :type "Float (single-precision)"))
  (switch `/Game/An/BluePrint/EnumEnemy` (`self.State`)
    (:`NewEnumerator0`
      (`KismetSystemLibrary.PrintString` "Idle"))
    (:`NewEnumerator1`
      (`KismetSystemLibrary.PrintString` "Move")
      (`|AIMoveTo` self (0.0 0.0 0.0) (stale `self.Sphere.OnComponentBeginOverlap` OtherActor) 500.0
        (:`OnSuccess`
          _)
        (:`OnFail`
          _))
      (set `self.State` "NewEnumerator2"))
    (:`NewEnumerator2`
      ;[1 1 1] 공격
      (if (>= (`self.GetDistanceTo` (stale `self.Sphere.OnComponentBeginOverlap` OtherActor)) 700.0)
        (set `self.State` "NewEnumerator1")
        (else
          (`KismetSystemLibrary.PrintString` "attack!")
          (`self.Jump`))))))

(event `self.Sphere.OnComponentBeginOverlap`
  (params (OverlappedComponent :type "PrimitiveComponent Object Reference") (OtherActor :type "Actor Object Reference") (OtherComp :type "PrimitiveComponent Object Reference") (OtherBodyIndex :type Integer) (bFromSweep :type Boolean) (SweepResult :type "HitResult Structure (by ref)"))
  ;[1 1 1] 충돌시 Harry검증
  (if (== (`KismetStringLibrary.Conv_StringToName` (`KismetSystemLibrary.GetDisplayName` OtherActor)) "MYHarry")
    (set `self.State` "NewEnumerator1")))

(fn `UserConstructionScript`)
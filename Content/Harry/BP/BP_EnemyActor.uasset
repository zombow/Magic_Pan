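; BP_EnemyActor is an enemy actor meant to move and explode on contact with the player, but its logic is currently disconnected.
; BeginPlay, overlap and Tick are empty.
; Unwired nodes would pick a target or forward direction at random, translate along it, and on overlap spawn an emitter and destroy both actors.
; Translate is an empty stub, and GetTargetDirection returns a zero vector.
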(event `self.ReceiveBeginPlay`)

(event `self.ReceiveActorBeginOverlap`
  (params (OtherActor :type "Actor Object Reference"))
  ;[1 1 1] Enemy가 Player와 부딪혔다!!! : 너 죽고 - (폭발VFX)만들고 - `나 죽자!
)

(event `self.ReceiveTick`
  (params (DeltaSeconds :type "Float (single-precision)"))
  ;[1 1 1] 아래로 이동하고 싶다.
)

(fn `GetTargetDirection`
  (returns (NewParam :type "Vector Structure"))
  (return (0.0 0.0 0.0)))

(fn `Translate`
  (params (Direction :type "Vector Structure") (Speed :type "Float (double-precision)") (DetaSecond :type "Float (double-precision)")))

(fn `UserConstructionScript`)
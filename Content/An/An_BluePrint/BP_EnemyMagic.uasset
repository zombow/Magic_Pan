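; BP_EnemyMagic is an actor with a Sphere component that, going by its name, serves as an enemy magic attack.
; Its only live logic plays the IceSpell sound at its location on BeginPlay.
; Overlap and Tick events are empty, and no movement logic runs in the graph.
; Disconnected leftovers from what a Korean note calls a Fireball hold unused BP_Enemy casts, explosion effects, destruction, a timer and a zero impulse.
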(event `self.Sphere.OnComponentBeginOverlap`
  (params (OverlappedComponent :type "PrimitiveComponent Object Reference") (OtherActor :type "Actor Object Reference") (OtherComp :type "PrimitiveComponent Object Reference") (OtherBodyIndex :type Integer) (bFromSweep :type Boolean) (SweepResult :type "HitResult Structure (by ref)")))

(event `self.ReceiveActorBeginOverlap`
  (params (OtherActor :type "Actor Object Reference"))
  ;[1 1 1] 총알 (Fireball)이 Enemy와 부딪혔다!! 폭발 VFX만들고 Enemy 죽고 나 Fireball 죽자
)

(event `self.ReceiveBeginPlay`
  (`GameplayStatics.PlaySoundAtLocation` "/Game/An/An_sound/IceSpell.IceSpell" (`self.K2_GetActorLocation`) (struct) 1.0 1.0 0.0 null null null))

(fn `UserConstructionScript`)
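; Enemy Blueprint with a simple Move/Attack state machine run on Tick, with attack logic still a debug-print placeholder.
; A MyHarry actor entering the Sphere overlap switches it to Move, where AI MoveTo chases the overlapped actor.
; Move success or failure both switch to Attack, which reverts to Move once the target is too far away.
; The Idle print is unconnected.
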(event `self.ReceiveTick`
  (params (DeltaSeconds :type "Float (single-precision)"))
  (switch `/Game/An/An_BluePrint/EnumEnemy` (`self.State`)
    (:`NewEnumerator1`
      ;[1 1 1] 이동
      (`KismetSystemLibrary.PrintString` "Move")
      (`|AIMoveTo` self (0.0 0.0 0.0) (stale `self.Sphere.OnComponentBeginOverlap` OtherActor) 500.0
        (:`OnSuccess`
          _)
        (:`OnFail`
          _))
      (set `self.State` "NewEnumerator2"))
    (:`NewEnumerator2`
      ;[1 1 1] 공격
      (if (>= (`self.GetDistanceTo` (stale `self.Sphere.OnComponentBeginOverlap` OtherActor)) 1300.0)
        (set `self.State` "NewEnumerator1")
        (else
          ;[1 1 1] 공격 애니메이션 및 체력 시스템
          (`KismetSystemLibrary.PrintString` "attack!"))))))

(event `self.Sphere.OnComponentBeginOverlap`
  (params (OverlappedComponent :type "PrimitiveComponent Object Reference") (OtherActor :type "Actor Object Reference") (OtherComp :type "PrimitiveComponent Object Reference") (OtherBodyIndex :type Integer) (bFromSweep :type Boolean) (SweepResult :type "HitResult Structure (by ref)"))
  ;[1 1 1] 충돌시 Harry검증
  (cast `/Game/ThirdPersonBP/Blueprints/MyHarry` OtherActor)
  (set `self.State` "NewEnumerator1"))

(fn `UserConstructionScript`)
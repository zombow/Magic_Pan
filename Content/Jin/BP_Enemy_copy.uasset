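; Enemy character Blueprint that can turn to face player 0 and stores an overlapping MyHarry as its target.
; Tick smoothly rotates it while FacePlayer is set by the face-player events; sphere overlap sets State to Move.
; An Idle/Move/Attack state switch using AI MoveTo and random normal or stab attack flags on En_AnimBlueprint is present but disconnected, as is the walk-speed setup.
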(event `FacePlayers`
  (set `self.FacePlayer` true))

(event `StopFacePlyers`
  (set `self.FacePlayer` false))

(event `self.ReceiveBeginPlay`
  ;[1 1 1] 캐릭터 이동속도 조정
)

(event `self.ReceiveTick`
  (params (DeltaSeconds :type "Float (single-precision)"))
  ;[1 1 1] State 분기
  (set `self.delta` DeltaSeconds)
  (if (`self.FacePlayer`)
    (`self.K2_SetActorRotation` (`KismetMathLibrary.RInterpTo` (`self.K2_GetActorRotation`) (`KismetMathLibrary.FindLookAtRotation` (`self.K2_GetActorLocation`) (`self.K2_GetActorLocation` (`GameplayStatics.GetPlayerCharacter` 0))) (`self.delta`) 2.0))))

(event `self.Sphere.OnComponentBeginOverlap`
  (params (OverlappedComponent :type "PrimitiveComponent Object Reference") (OtherActor :type "Actor Object Reference") (OtherComp :type "PrimitiveComponent Object Reference") (OtherBodyIndex :type Integer) (bFromSweep :type Boolean) (SweepResult :type "HitResult Structure (by ref)"))
  ;[1 1 1] 충돌시 Harry검증
  (bind _asmy_harry (cast `/Game/ThirdPersonBP/Blueprints/MyHarry` OtherActor))
  (set `self.player` _asmy_harry)
  (set `self.State` "NewEnumerator1"))

(fn `Cast enemy bool`
  (returns (enemyAttack :type Boolean) (enemystabAttack :type Boolean))
  (bind _asen_anim_blueprint (cast `/Game/An/An_animations/En_AnimBlueprint` (`SkeletalMeshComponent.GetAnimInstance` (`self.Mesh`))))
  (return (`/Game/An/An_animations/En_AnimBlueprint.bAttack` _asen_anim_blueprint) (`/Game/An/An_animations/En_AnimBlueprint.stabAttack` _asen_anim_blueprint)))

(fn `Oder Attack`
  (params (attackState :type Boolean))
  (bind _asen_anim_blueprint (cast `/Game/An/An_animations/En_AnimBlueprint` (`SkeletalMeshComponent.GetAnimInstance` (`self.Mesh`))))
  (if (> (`KismetMathLibrary.RandomFloatInRange` 0.0 1.0) 0.4)
    (set `/Game/An/An_animations/En_AnimBlueprint.bAttack` attackState _asen_anim_blueprint)
    (else
      (set `/Game/An/An_animations/En_AnimBlueprint.stabAttack` attackState _asen_anim_blueprint))))

(fn `UserConstructionScript`)